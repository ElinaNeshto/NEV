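; Player character Blueprint for NEV that lets the player pick up or equip weapons from interactable actors.
; On the interact input, it takes a short-range aim point hit and calls InteractMessage on actors implementing BPI_Interactable.
; A valid returned class becomes the WeaponComponent's weapon class, and the component is reinitialized.
; BeginPlay and the construction script are empty, and a debug sphere trace is left unconnected.
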(event Input|EnhancedActionEvents|EnhancedInputActionIA_NEVInteract
  (params (ActionValue :type Boolean) (ElapsedSeconds :type Float%20%28double-precision%29) (TriggeredSeconds :type Float%20%28double-precision%29) (InputAction :type Input%20Action%20Object%20Reference :default "/Game/NEV/Input/Actions/IA_NEVInteract.IA_NEVInteract"))
  (bind _hitresult (Class|NEVBaseCharacter|GetAimPoint 5e+02))
  (bind (_bblockinghit _binitialoverlap _time _distance _location _impactpoint _normal _impactnormal _physmat _hitactor) (Collision|BreakHitResult _hitresult))
  (if _bblockinghit
    (if (Utilities|DoesObjectImplementInterface _hitactor "/Game/NEV/Interfaces/BPI_Interactable.BPI_Interactable_C")
      (bind _actor (Class|BPIInteractable|Interact(Message) _hitactor))
      (if (Utilities|IsValidClass _actor)
        (Variables|/Script/NEV.NEVWeaponComponent|SetWeaponClass (Variables|Default|GetWeaponComponent) _actor)
        (Class|NEVWeaponComponent|InitWeaponComponent (Variables|Default|GetWeaponComponent))))))

(event EventBeginPlay)

(fn ConstructionScript)